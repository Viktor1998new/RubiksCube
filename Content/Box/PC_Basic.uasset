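; Player controller for a match-based box game, handling each player's spawn, HUD and match-state transitions.
; On begin play it initializes networking through PS_Basic, creates the W_Game widget in waiting state and passes the saved skin to GM_Game for spawning.
; Start, stop, victory and Escape-menu events switch widget state, cursor and input mode.
; Ready state goes through PS_Basic; game results and wins are recorded in My_Instence.
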(event `self.ReceiveBeginPlay`
  (`self.Cliend_Init`))

(event `Cliend_Init`
  (`self.Init_Net`)
  (bind _returnvalue (`|CreateWidget` "/Game/Box/Widgets/W_Game.W_Game_C" self))
  (set `self.Game_widget` _returnvalue)
  (`/Game/Box/Widgets/W_Game.IsWait` (`self.Game_widget`) true)
  (set `self.bShowMouseCursor` true)
  (bind _asmy_instence (cast `/Game/My_Instence` (`GameplayStatics.GetGameInstance`)))
  (`self.Send_Spawn` (`/Game/My_Instence.Skin` _asmy_instence))
  (`UserWidget.AddToViewport` (`self.Game_widget`) 0)
  (`WidgetBlueprintLibrary.SetInputMode_UIOnlyEx` self (`self.Game_widget`))
  (`Widget.SetKeyboardFocus` (`self.Game_widget`)))

(event `Init_Net`
  (bind _asps_basic (cast `/Game/Box/PS_Basic` (`self.PlayerState`)))
  (`/Game/Box/PS_Basic.Send_Net` _asps_basic))

(event `StartGame`
  (`/Game/Box/Widgets/W_Game.IsWait` (`self.Game_widget`) false)
  (set `self.bShowMouseCursor` false)
  (`WidgetBlueprintLibrary.SetInputMode_GameOnly` self)
  (bind _asps_basic (cast `/Game/Box/PS_Basic` (`self.PlayerState`)))
  (`/Game/Box/PS_Basic.Send_Ready` _asps_basic false))

(event `Key|Escape`
  (params (Key :type "Key Structure"))
  (bind _game_widget (`self.Game_widget`))
  (:`Pressed`
    (`/Game/Box/Widgets/W_Game.Menu` _game_widget)
    (if (`/Game/Box/Widgets/W_Game.IsMenu` _game_widget)
      (set `self.bShowMouseCursor` true)
      (`WidgetBlueprintLibrary.SetInputMode_UIOnlyEx` self (`self.Game_widget`))
      (`Widget.SetKeyboardFocus` (`self.Game_widget`))
      (else
        (set `self.bShowMouseCursor` false)
        (`WidgetBlueprintLibrary.SetInputMode_GameOnly` self)))))

(event `StopGame`
  (`/Game/Box/Widgets/W_Game.IsWait` (`self.Game_widget`) true)
  (set `self.bShowMouseCursor` true)
  (`WidgetBlueprintLibrary.SetInputMode_UIOnlyEx` self (`self.Game_widget`)))

(event `Send_VictotyPlayer`
  (params (Player :type "/Game/Box/PS_Basic Object Reference"))
  (`/Game/Box/Widgets/W_Game.WinPlayer` (`self.Game_widget`) Player)
  (set `self.bShowMouseCursor` true)
  (`WidgetBlueprintLibrary.SetInputMode_UIOnlyEx` self (`self.Game_widget`))
  (bind _asmy_instence (cast `/Game/My_Instence` (`GameplayStatics.GetGameInstance`)))
  (`/Game/My_Instence.AddGame` _asmy_instence false))

(event `Send_Spawn`
  (params (BoxSkin :type Name))
  (set `self.Box Skin` BoxSkin)
  (bind _asgm_game (cast `/Game/Box/GM_Game` (`GameplayStatics.GetGameMode`)))
  (`/Game/Box/GM_Game.SpawnBox` _asgm_game self (`self.Box Skin`)))

(event `AddVictory`
  (bind _asmy_instence (cast `/Game/My_Instence` (`GameplayStatics.GetGameInstance`)))
  (`/Game/My_Instence.AddGame` _asmy_instence true))

(event `Ready`
  (bind _asps_basic (cast `/Game/Box/PS_Basic` (`self.PlayerState`)))
  (`/Game/Box/PS_Basic.Ready` _asps_basic))

(fn `UserConstructionScript`)