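; GM_Game is a game mode for a box game, declaring hooks for player readiness, box spawning and player victory, all empty here.
; Its only implemented logic, Confuse, reseeds a random stream and builds a list of random AI structs, apparently scramble moves.
; Each entry holds a column and row on a three-by-three range plus a Back flag, one per loop index up to LastIndex.
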(fn `Confuse`
  (params (LastIndex :type Integer))
  (returns (ReturnValue :type "Array of /Game/Box/AIStruct Structure"))
  (locals (L_Steam :type "RandomStream Structure") (L_Return :type "Array of /Game/Box/AIStruct Structure"))
  (`KismetMathLibrary.SeedRandomStream` (`local.L_Steam`))
  (for _ (range (+ LastIndex 1))
    (`KismetArrayLibrary.Array_Add` (`local.L_Return`) (make `/Game/Box/AIStruct` (`KismetMathLibrary.RandomIntegerInRangeFromStream` 0 2 (`local.L_Steam`)) (`KismetMathLibrary.RandomIntegerInRangeFromStream` 0 2 (`local.L_Steam`)) (`KismetMathLibrary.RandomBoolFromStream` (`local.L_Steam`)))))
  (return (`local.L_Return`)))

(fn `ReadyPlayer`
  (params (NewEnable :type Boolean)))

(fn `SpawnBox`
  (params (Player :type "/Game/Box/PC_Basic Object Reference") (Skin :type Name)))

(fn `UserConstructionScript`)

(fn `VictoryPlayer`
  (params (Player :type "/Game/Box/PC_Basic Object Reference")))