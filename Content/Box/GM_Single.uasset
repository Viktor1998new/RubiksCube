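; Single-player game mode for a box-rotation puzzle that scrambles the player's box and supplies a new one after each win.
; SpawnBox spawns a skinned Pawn_Box_Player in a grid position derived from a running pawn count, then possesses it.
; Wins preserve control rotation across the pawn swap.
; Start, restart and win paths replay move lists from Confuse through ServerRotate, using either a random count or LastIndex.
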(event `RestatrGame`
  (bind _returnvalue (`self.Confuse` (`KismetMathLibrary.RandomIntegerInRange` 100 500)))
  (for _array_element _returnvalue
    (bind (_column _row _back) (break `/Game/Box/AIStruct` _array_element))
    (`/Game/Box/Pawn_Box.Server_Rotate` (`self.Box_Pawn`) _column _row _back false))
  (set `/Game/Box/Pawn_Box.IsStart` true (`self.Box_Pawn`)))

(event `WInPlayer`
  (params (Player :type "/Game/Box/PC_Basic Object Reference"))
  (bind _player (`self.Player`))
  (set `self.Pawns` (+ (`self.Pawns`) 1))
  (set `self.ControllerRotate` (`Controller.GetControlRotation` (`self.Player`)))
  (`self.SpawnBox` _player (`/Game/Box/PC_Basic.Box Skin` _player))
  (`Controller.SetControlRotation` (`self.Player`) (`self.ControllerRotate`))
  (set `/Game/Box/Pawn_Box.IsStart` true (`self.Box_Pawn`))
  (bind _returnvalue (`self.Confuse` (`KismetMathLibrary.RandomIntegerInRange` 100 500)))
  (for _array_element _returnvalue
    (bind (_column _row _back) (break `/Game/Box/AIStruct` _array_element))
    (`/Game/Box/Pawn_Box.Server_Rotate` (`self.Box_Pawn`) _column _row _back false)))

(fn `ReadyPlayer`
  (params (NewEnable :type Boolean))
  (if NewEnable
    (`/Game/Box/PC_Basic.StartGame` (`self.Player`))
    (set `/Game/Box/Pawn_Box.IsStart` true (`self.Box_Pawn`))
    (bind _returnvalue (`self.Confuse` (`self.Last Index`)))
    (for _array_element _returnvalue
      (bind (_column _row _back) (break `/Game/Box/AIStruct` _array_element))
      (`/Game/Box/Pawn_Box.Server_Rotate` (`self.Box_Pawn`) _column _row _back false))))

(fn `SpawnBox`
  (params (Player :type "/Game/Box/PC_Basic Object Reference") (Skin :type Name))
  (bind _pawns (`self.Pawns`))
  (set `self.Player` Player)
  (bind _returnvalue (`|SpawnActorFromClass` "/Game/Box/Pawn_Box_Player.Pawn_Box_Player_C" (`KismetMathLibrary.MakeTransform` (`KismetMathLibrary.MakeVector` (* (/ _pawns 10) -400.0) (* (mod _pawns 10) 400.0))) "AlwaysSpawn" "OverrideRootScale" Player Skin null))
  (`Controller.Possess` Player _returnvalue)
  (set `self.Box_Pawn` _returnvalue))

(fn `UserConstructionScript`)

(fn `VictoryPlayer`
  (params (Player :type "/Game/Box/PC_Basic Object Reference"))
  (bind _player (`self.Player`))
  (set `self.Pawns` (+ (`self.Pawns`) 1))
  (set `self.ControllerRotate` (`Controller.GetControlRotation` (`self.Player`)))
  (`self.SpawnBox` _player (`/Game/Box/PC_Basic.Box Skin` _player))
  (`Controller.SetControlRotation` (`self.Player`) (`self.ControllerRotate`))
  (set `/Game/Box/Pawn_Box.IsStart` true (`self.Box_Pawn`))
  (bind _returnvalue (`self.Confuse` (`self.Last Index`)))
  (for _array_element _returnvalue
    (bind (_column _row _back) (break `/Game/Box/AIStruct` _array_element))
    (`/Game/Box/Pawn_Box.Server_Rotate` (`self.Box_Pawn`) _column _row _back false)))