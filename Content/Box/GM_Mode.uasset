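; Game mode for the multiplayer Box puzzle race, handling ready-up, spawning, victory and restarts.
; When all players, at least two, are ready, it flags the session begun and sends every box one shared random scramble.
; The first finisher wins and starts a countdown; timeout or everyone finishing announces the winner, credits public-match victories and schedules a restart.
; Restarts, or logouts leaving one player, respawn boxes on a grid and reopen the session.
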(event `self.K2_PostLogin`
  (params (NewPlayer :type "PlayerController Object Reference"))
  (bind _aspc_basic (cast `/Game/Box/PC_Basic` NewPlayer))
  (`KismetArrayLibrary.Array_Add` (`self.Players`) _aspc_basic))

(event `Send_Start`
  (bind _returnvalue (`self.Confuse` (`KismetMathLibrary.RandomIntegerInRange` 100 500)))
  (bind _outactors (`GameplayStatics.GetAllActorsOfClass` "/Game/Box/Pawn_Box.Pawn_Box_C"))
  (for _array_element _outactors
    (for _array_element_2 _returnvalue
      (bind (_column _row _back) (break `/Game/Box/AIStruct` _array_element_2))
      (`/Game/Box/Pawn_Box.Server_Rotate` _array_element _column _row _back false))))

(event `EndGame`
  (`UpdateSessionCallbackProxyAdvanced.UpdateSession` (`|MakeArray` (`AdvancedSessionsLibrary.MakeLiteralSessionPropertyString` "Game" "Box") (`AdvancedSessionsLibrary.MakeLiteralSessionPropertyBool` "Private" (`self.IsPrivate`)) (`AdvancedSessionsLibrary.MakeLiteralSessionPropertyBool` "Begin")) (`self.MaxPlayer`)))

(event `BeginGame`
  (`UpdateSessionCallbackProxyAdvanced.UpdateSession` (`|MakeArray` (`AdvancedSessionsLibrary.MakeLiteralSessionPropertyString` "Game" "Box") (`AdvancedSessionsLibrary.MakeLiteralSessionPropertyBool` "Private" (`self.IsPrivate`)) (`AdvancedSessionsLibrary.MakeLiteralSessionPropertyBool` "Begin" true)) (`self.MaxPlayer`)
    (:`OnSuccess`
      _)
    (:`OnFailure`
      _))
  (for _array_element (`self.Players`)
    (`/Game/Box/PC_Basic.StartGame` _array_element))
  (bind _outactors (`GameplayStatics.GetAllActorsOfClass` "/Game/Box/Pawn_Box.Pawn_Box_C"))
  (for _array_element_2 _outactors
    (set `/Game/Box/Pawn_Box.IsStart` true _array_element_2))
  (`KismetSystemLibrary.Delay` 0.2)
  (`self.Send_Start`)
  (set `self.Player_Ready` 0))

(event `self.ReceiveBeginPlay`
  (bind _numconnections (`AdvancedSessionsLibrary.GetSessionSettings`)
    (:`OnSuccess`
      (set `self.MaxPlayer` _numconnections))))

(event `RestatrGame`
  (set `self.Player_Victory` null)
  (set `self.Player_End` 0)
  (`UpdateSessionCallbackProxyAdvanced.UpdateSession` (`|MakeArray` (`AdvancedSessionsLibrary.MakeLiteralSessionPropertyString` "Game" "Box") (`AdvancedSessionsLibrary.MakeLiteralSessionPropertyBool` "Private") (`AdvancedSessionsLibrary.MakeLiteralSessionPropertyBool` "Begin")) (`self.MaxPlayer`)
    (:`then`
      (for _array_element (`self.Players`)
        (`self.K2_DestroyActor` (`Controller.K2_GetPawn` _array_element))
        (`self.SpawnBox` _array_element (`/Game/Box/PC_Basic.Box Skin` _array_element))))))

(event `self.K2_OnLogout`
  (params (ExitingController :type "Controller Object Reference"))
  (bind _output (`|GetArrayItem` (`self.Players`)))
  (bind _aspc_basic (cast `/Game/Box/PC_Basic` ExitingController))
  (`KismetArrayLibrary.Array_RemoveItem` (`self.Players`) _aspc_basic)
  (bind _asgs_basic (cast `/Game/Box/GS_Basic` (`GameplayStatics.GetGameState`)))
  (`/Game/Box/GS_Basic.RemovePlayer` _asgs_basic (cast `/Game/Box/PS_Basic` (`Controller.PlayerState` _aspc_basic) :!pure true))
  (if (== (`KismetArrayLibrary.Array_Length` (`self.Players`)) 1)
    (`/Game/Box/PC_Basic.StopGame` _output)
    (`self.K2_DestroyActor` (`Controller.K2_GetPawn` _output))
    (`self.SpawnBox` _output (`/Game/Box/PC_Basic.Box Skin` _output))
    (`UpdateSessionCallbackProxyAdvanced.UpdateSession` (`|MakeArray` (`AdvancedSessionsLibrary.MakeLiteralSessionPropertyString` "Game" "Box") (`AdvancedSessionsLibrary.MakeLiteralSessionPropertyBool` "Private") (`AdvancedSessionsLibrary.MakeLiteralSessionPropertyBool` "Begin")) (`self.MaxPlayer`))))

(event `StartTimerEndGame`
  (bind _returnvalue (`KismetSystemLibrary.K2_SetTimerDelegate` (delegate `Event_EndGame`) (`KismetMathLibrary.GetTotalSeconds` (`KismetMathLibrary.MakeTimespan` 0 0 0 30))))
  (set `self.TimerEndGame` _returnvalue))

(event `Event_EndGame`
  (for _array_element (`self.Players`)
    (bind _aspawn_box (cast `/Game/Box/Pawn_Box` (`Controller.K2_GetPawn` _array_element)))
    (set `/Game/Box/Pawn_Box.IsStart` false _aspawn_box)
    (if (!= _array_element (`self.Player_Victory`))
      (`/Game/Box/PC_Basic.Send_VictotyPlayer` _array_element (cast `/Game/Box/PS_Basic` (`Controller.PlayerState` (`self.Player_Victory`)) :!pure true))))
  (`/Game/Box/PC_Basic.Send_VictotyPlayer` (`self.Player_Victory`) (cast `/Game/Box/PS_Basic` (`Controller.PlayerState` (`self.Player_Victory`)) :!pure true))
  (`|ExecutionSequence`
    (:`then_0`
      (if (not (`self.IsPrivate`))
        (`/Game/Box/PC_Basic.AddVictory` (`self.Player_Victory`))))
    (:`then_1`
      (`self.EndGame`)
      (`self.TimerRestartGame`))))

(event `TimerRestartGame`
  (`KismetSystemLibrary.K2_SetTimerDelegate` (delegate `Event_RestartGame`) (`KismetMathLibrary.GetTotalSeconds` (`KismetMathLibrary.MakeTimespan` 0 0 0 15))))

(event `Event_RestartGame`
  (`self.RestatrGame`)
  (for _array_element (`self.Players`)
    (`/Game/Box/PC_Basic.StopGame` _array_element)))

(fn `ReadyPlayer`
  (params (NewEnable :type Boolean))
  (bind _player_ready (`self.Player_Ready`))
  (bind _returnvalue (`KismetArrayLibrary.Array_Length` (`self.Players`)))
  (if NewEnable
    (set `self.Player_Ready` (+ _player_ready 1))
    (else
      (set `self.Player_Ready` (- _player_ready 1))))
  (if (and (== (`self.Player_Ready`) _returnvalue) (> _returnvalue 1))
    (`self.BeginGame`)))

(fn `SpawnBox`
  (params (Player :type "/Game/Box/PC_Basic Object Reference") (Skin :type Name))
  (bind _pawns (`self.Pawns`))
  (set `self.Pawns` (+ (`self.Pawns`) 1))
  (bind _returnvalue (`|SpawnActorFromClass` "/Game/Box/Pawn_Box_Player.Pawn_Box_Player_C" (`KismetMathLibrary.MakeTransform` (`KismetMathLibrary.MakeVector` (* (/ _pawns 10) -400.0) (* (mod _pawns 10) 400.0))) "AlwaysSpawn" "OverrideRootScale" Player Skin null))
  (`Controller.Possess` Player _returnvalue))

(fn `UserConstructionScript`)

(fn `VictoryPlayer`
  (params (Player :type "/Game/Box/PC_Basic Object Reference"))
  (bind _player_victory (`self.Player_Victory`))
  (bind _output_get (set `self.Player_End` (+ (`self.Player_End`) 1)))
  (if (== _output_get (`KismetArrayLibrary.Array_Length` (`self.Players`)))
    (`KismetSystemLibrary.K2_ClearAndInvalidateTimerHandle` (`self.TimerEndGame`))
    (for _array_element (`self.Players`)
      (if (!= _array_element (`self.Player_Victory`))
        (`/Game/Box/PC_Basic.Send_VictotyPlayer` _array_element (cast `/Game/Box/PS_Basic` (`Controller.PlayerState` (`self.Player_Victory`)) :!pure true))))
    (`/Game/Box/PC_Basic.Send_VictotyPlayer` _player_victory (cast `/Game/Box/PS_Basic` (`Controller.PlayerState` _player_victory) :!pure true))
    (`|ExecutionSequence`
      (:`then_0`
        (if (not (`self.IsPrivate`))
          (`/Game/Box/PC_Basic.AddVictory` (`self.Player_Victory`))))
      (:`then_1`
        (`self.EndGame`)
        (`self.TimerRestartGame`)))
    (elif (== _output_get 1)
      (set `self.Player_Victory` Player)
      (`self.StartTimerEndGame`))))